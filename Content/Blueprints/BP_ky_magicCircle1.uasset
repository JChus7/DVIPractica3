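; BP_ky_magicCircle1 is a magic circle that spawns enemy AI pawns inside its box.
; Each call to Spawn uses TipoSpawn to pick a swordman or mage at a random point in the box, or a skeleton king at its center, then decrements NumeroSpawns until none remain.
; The construction script passes the Color variable to the Fx effect's color parameter.
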(event `Spawn`
  (bind _box (`self.Box`))
  (bind _returnvalue (`SceneComponent.K2_GetComponentLocation` _box))
  (bind _returnvalue_2 (`KismetMathLibrary.RandomPointInBoundingBox` _returnvalue (`BoxComponent.GetScaledBoxExtent` _box)))
  (if (> (`self.Numero spawns`) 0)
    (switch `int` (`self.Tipo spawn`)
      (:`0`
        (`AIBlueprintHelperLibrary.SpawnAIFromClass` "/Game/Blueprints/Swordman_Blueprint.Swordman_Blueprint_C" null _returnvalue_2))
      (:`1`
        (`AIBlueprintHelperLibrary.SpawnAIFromClass` "/Game/Blueprints/Mago_Blueprint.Mago_Blueprint_C" null _returnvalue_2))
      (:`2`
        (`AIBlueprintHelperLibrary.SpawnAIFromClass` "/Game/Blueprints/ReyEsqueleto_Blueprint.ReyEsqueleto_Blueprint_C" null _returnvalue (struct :`Yaw` 180.0))))
    (bind _result (`/Engine/EditorBlueprintResources/StandardMacros.DecrementInt` (`self.Numero spawns`))
      (:`  `
        (set `self.Numero spawns` _result)))))

(fn `UserConstructionScript`
  (`parent.UserConstructionScript`)
  (`ParticleSystemComponent.SetVectorParameter` (`self.fx`) "color" (`KismetMathLibrary.Conv_LinearColorToVector` (`self.color`))))